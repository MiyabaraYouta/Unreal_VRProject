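; Test Blueprint that drives an Arduino over a serial COM port with zone-and-strength text commands, apparently for fans.
; BeginPlay enables input, opens the port and prints the result, and EndPlay closes it.
; SendSerial maps a FunStrong value (all, right, center or left at five levels, plus stop) to a string, then sends and prints it.
; Number-key presses trigger a few sample commands.
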(event `self.ReceiveBeginPlay`
  (`self.EnableInput` (`GameplayStatics.GetPlayerController` 0))
  (bind (_bopened _returnvalue) (`Serial.OpenComPort` 3 115200))
  (set `self.Ardino` _returnvalue)
  (bind _output_get (set `self.Opened` _bopened))
  (if _output_get
    (`KismetSystemLibrary.PrintString` "OpenPort")
    (else
      (`KismetSystemLibrary.PrintString` "NoOpen"))))

(event `self.ReceiveEndPlay`
  (params (EndPlayReason :type "EEndPlayReason Enum" :default "Destroyed"))
  (`Serial.Close` (`self.Ardino`)))

(event `Key|Six`
  (params (Key :type "Key Structure"))
  (:`Pressed`
    (`self.SendSerial` "NewEnumerator0")))

(event `Key|Eight`
  (params (Key :type "Key Structure"))
  (:`Pressed`
    (`self.SendSerial` "NewEnumerator10")))

(event `Key|Seven`
  (params (Key :type "Key Structure"))
  (:`Pressed`
    (`self.SendSerial` "NewEnumerator5")))

(event `Key|Nine`
  (params (Key :type "Key Structure"))
  (:`Pressed`
    (`self.SendSerial` "NewEnumerator15")))

(event `Key|Zero`
  (params (Key :type "Key Structure"))
  (:`Pressed`
    (`self.SendSerial` "NewEnumerator4")))

(event `/Game/BluePrints/ITurnAngle.GetPlayerTurnAngle`
  (params (_turnAngle :type "Float (double-precision)")))

(fn `SendSerial`
  (params (Fun_Strong :type "/Game/BluePrints/Audino/Fun_string Enum" :default "NewEnumerator0"))
  (switch `/Game/BluePrints/Audino/Fun_string` Fun_Strong
    (:`NewEnumerator0`
      (set `self.Input` "all_5"))
    (:`NewEnumerator1`
      (set `self.Input` "all_4"))
    (:`NewEnumerator2`
      (set `self.Input` "all_3"))
    (:`NewEnumerator3`
      (set `self.Input` "all_2"))
    (:`NewEnumerator4`
      (set `self.Input` "all_1"))
    (:`NewEnumerator5`
      (set `self.Input` "right_5"))
    (:`NewEnumerator6`
      (set `self.Input` "right_4"))
    (:`NewEnumerator7`
      (set `self.Input` "right_3"))
    (:`NewEnumerator8`
      (set `self.Input` "right_2"))
    (:`NewEnumerator9`
      (set `self.Input` "right_1"))
    (:`NewEnumerator10`
      (set `self.Input` "center_5"))
    (:`NewEnumerator11`
      (set `self.Input` "center_4"))
    (:`NewEnumerator12`
      (set `self.Input` "Center_3"))
    (:`NewEnumerator13`
      (set `self.Input` "center_2"))
    (:`NewEnumerator14`
      (set `self.Input` "center_1"))
    (:`NewEnumerator15`
      (set `self.Input` "left_5"))
    (:`NewEnumerator16`
      (set `self.Input` "left_4"))
    (:`NewEnumerator17`
      (set `self.Input` "left_3"))
    (:`NewEnumerator18`
      (set `self.Input` "left_2"))
    (:`NewEnumerator19`
      (set `self.Input` "left_1"))
    (:`NewEnumerator20`
      (set `self.Input` "")))
  (`Serial.Print` (`self.Ardino`) (`self.Input`))
  (`Serial.LineEndToStr` (`self.Ardino`) "n")
  (`KismetSystemLibrary.PrintString` (`self.Input`)))

(fn `UserConstructionScript`)