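; BP_DeviceTest is a VR debug Blueprint that shows live motion controller readings on screen.
; Each Tick it reads both hands through GetMotionControllerData, storing aim height (Z) and a rotation approximated as the aim quaternion's X times 90.
; It prints the stored values before updating them, so the display trails by one frame.
; A similar HMD head-rotation readout exists but is disconnected and never runs.
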(event `self.ReceiveTick`
  (params (DeltaSeconds :type "Float (single-precision)"))
  (`|ExecutionSequence`
    (:`then_0`
      ;[1 1 1] Output Right Aim Rotation and RightHeight
      (bind _motioncontrollerdata (`HeadMountedDisplayFunctionLibrary.GetMotionControllerData` "/Game/VRTemplate/Blueprints/VRPawn.VRPawn" "Right"))
      (`|ExecutionSequence`
        (:`then_0`
          (`KismetSystemLibrary.PrintString` (`KismetStringLibrary.Concat_StrStr` "RightHandRelativeHeght" (`KismetStringLibrary.Conv_DoubleToString` (stale _output_get)) "RightRotation" (`KismetStringLibrary.Conv_DoubleToString` (stale _output_get_2))) true true (struct :`A` 1.0) DeltaSeconds))
        (:`then_1`
          (bind _output_get (set `self.RightHandRelativeHeight` (.z (`.AimPosition` (break `XRMotionControllerData` _motioncontrollerdata))))))
        (:`then_2`
          (bind _output_get_2 (set `self.RightArmRotation` (* (`KismetMathLibrary.BreakQuat` (`.AimRotation` (break `XRMotionControllerData` _motioncontrollerdata))) 90.0))))))
    (:`then_1`
      ;[1 1 1] Output Left Aim Rotation and Left Height
      (bind _motioncontrollerdata_2 (`HeadMountedDisplayFunctionLibrary.GetMotionControllerData` "/Game/VRTemplate/Blueprints/VRPawn.VRPawn" "Left"))
      (`|ExecutionSequence`
        (:`then_0`
          (`KismetSystemLibrary.PrintString` (`KismetStringLibrary.Concat_StrStr` "LeftHandRelativeHeight" (`KismetStringLibrary.Conv_DoubleToString` (stale _output_get_3)) "LeftRotation" (`KismetStringLibrary.Conv_DoubleToString` (stale _output_get_4))) true true (struct :`A` 1.0) DeltaSeconds))
        (:`then_1`
          (bind _output_get_3 (set `self.LeftHandRelativeHeight` (.z (`.AimPosition` (break `XRMotionControllerData` _motioncontrollerdata_2))))))
        (:`then_2`
          (bind _output_get_4 (set `self.LeftArmRotation` (* (`KismetMathLibrary.BreakQuat` (`.AimRotation` (break `XRMotionControllerData` _motioncontrollerdata_2))) 90.0))))))
    (:`then_2`)))

(fn `UserConstructionScript`)