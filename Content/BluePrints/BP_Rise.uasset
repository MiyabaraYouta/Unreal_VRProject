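; BP_Rise is an Actor Blueprint that pushes the VR pawn upward when both motion controllers swing down quickly, like a flapping gesture.
; Each Tick it derives each controller's vertical speed from the change in its aim component's relative Z over delta time.
; When both speeds pass a downward threshold, it applies an upward impulse to the VRPawn's capsule and prints a debug string.
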(event `self.ReceiveTick`
  (params (DeltaSeconds :type "Float (single-precision)"))
  (`|ExecutionSequence`
    (:`then_0`
      ;[1 1 1] コントローラーの移動量を取得する
      (bind _asvrpawn (cast `/Game/VRTemplate/Blueprints/VRPawn` (`GameplayStatics.GetPlayerPawn` 0)))
      (`|ExecutionSequence`
        (:`then_0`
          (bind (_relativelocation_x _relativelocation_y _relativelocation_z) (`KismetMathLibrary.BreakVector` (`SceneComponent.RelativeLocation` (`/Game/VRTemplate/Blueprints/VRPawn.MotionControllerLeftAim` _asvrpawn))))
          (set `self.LeftMovementZ` (/ (- _relativelocation_z (`self.LeftPositionZ`)) DeltaSeconds)))
        (:`then_1`
          (set `self.LeftPositionZ` _relativelocation_z))
        (:`then_2`
          (bind (_relativelocation_x_2 _relativelocation_y_2 _relativelocation_z_2) (`KismetMathLibrary.BreakVector` (`SceneComponent.RelativeLocation` (`/Game/VRTemplate/Blueprints/VRPawn.MotionControllerRightAim` _asvrpawn))))
          (set `self.RightMovementZ` (/ (- _relativelocation_z_2 (`self.RightPositionZ`)) DeltaSeconds)))
        (:`then_3`
          (set `self.RightPositionZ` _relativelocation_z_2))))
    (:`then_1`
      ;[1 1 1] コントローラーの移動量をもとに上昇させる
      (if (and (< (`self.LeftMovementZ`) -50.0) (< (`self.RightMovementZ`) -50.0))
        (bind _asvrpawn_2 (cast `/Game/VRTemplate/Blueprints/VRPawn` (`GameplayStatics.GetPlayerPawn` 0)))
        (`KismetSystemLibrary.PrintString` "Hello" true true (struct :`R` 1.0 :`B` 0.13627 :`A` 1.0) DeltaSeconds)
        (`PrimitiveComponent.AddImpulse` (`/Game/VRTemplate/Blueprints/VRPawn.Capsule` _asvrpawn_2) (0.0 0.0 100.0) "None" false)))))

(fn `UserConstructionScript`)