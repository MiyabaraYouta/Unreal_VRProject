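; VR flight tutorial that steps the player through holding still, flapping, turning left and turning right, then fades and opens the Sougen level.
; Tick runs a state machine, with delays pacing checks and transitions.
; Gestures are read from VRPawn motion controllers: per-call height change for stillness and flapping, hand-to-hand tilt angle for turns.
; Each success updates image state on two widgets, with a text widget following the first three steps.
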(event `self.ReceiveBeginPlay`
  (set `self.state` "NewEnumerator1"))

(event `self.ReceiveTick`
  (params (DeltaSeconds :type "Float (single-precision)"))
  (switch `/Game/BluePrints/TutorialState` (`self.state`)
    (:`NewEnumerator1`
      (`self.StateT`))
    (:`NewEnumerator2`
      (`self.StateFlap`))
    (:`NewEnumerator3`
      (`self.StateTurnLeft`))
    (:`NewEnumerator4`
      (`self.StateTurnRight`))))

(event `StateT`
  (bind _astutorial_ui (cast `/Game/BluePrints/TutorialUI` (`WidgetComponent.GetUserWidgetObject` (`self.Widget`))))
  (bind _astutorial_side (cast `/Game/BluePrints/tutorial_side` (`WidgetComponent.GetUserWidgetObject` (`self.Widgetside`))))
  (`|ExecutionSequence`
    (:`then_0`
      (`KismetSystemLibrary.Delay` 3.0)
      (bind _newparam (`self.Dont Move`))
      (set `self.dontmove` _newparam))
    (:`then_1`
      (if (`self.dontmove`)
        (`/Game/BluePrints/TutorialUI.ChangeImageState` _astutorial_ui "NewEnumerator1")
        (`/Game/BluePrints/tutorial_side.ChangeImageState` _astutorial_side "NewEnumerator1")
        (`KismetSystemLibrary.Delay` 2.0)
        (`/Game/BluePrints/TutorialUI.ChangeImageState` _astutorial_ui "NewEnumerator0")
        (`/Game/BluePrints/TutorialUI.ChangeImage` _astutorial_ui 1)
        (`/Game/BluePrints/tutorial_side.ChangeImageState` _astutorial_side "NewEnumerator0")
        (`/Game/BluePrints/tutorial_side.changeImage` _astutorial_side 1)
        (set `self.state` "NewEnumerator2")
        (bind _astutorial_text (cast `/Game/BluePrints/tutorial_text` (`WidgetComponent.GetUserWidgetObject` (`self.Widgettext`))))
        (`/Game/BluePrints/tutorial_text.changeText` _astutorial_text 1)))))

(event `StateFlap`
  (bind _astutorial_ui (cast `/Game/BluePrints/TutorialUI` (`WidgetComponent.GetUserWidgetObject` (`self.Widget`))))
  (bind _astutorial_side (cast `/Game/BluePrints/tutorial_side` (`WidgetComponent.GetUserWidgetObject` (`self.Widgetside`))))
  (`|ExecutionSequence`
    (:`then_0`
      (bind _newparam (`self.flap`))
      (set `self.flapflag` _newparam)
      (if (`self.roopflag`)
        (`KismetSystemLibrary.Delay` 0.5)
        (`self.callRoop3Image` 1 2 3)))
    (:`then_1`
      (if (`self.flapflag`)
        (`/Game/BluePrints/TutorialUI.ChangeImageState` _astutorial_ui "NewEnumerator1")
        (`/Game/BluePrints/tutorial_side.ChangeImageState` _astutorial_side "NewEnumerator1")
        (set `self.roopflag` false)
        (`KismetSystemLibrary.Delay` 2.0)
        (`/Game/BluePrints/TutorialUI.ChangeImageState` _astutorial_ui "NewEnumerator0")
        (`/Game/BluePrints/TutorialUI.ChangeImage` _astutorial_ui 4)
        (`/Game/BluePrints/tutorial_side.ChangeImageState` _astutorial_side "NewEnumerator0")
        (`/Game/BluePrints/tutorial_side.changeImage` _astutorial_side 4)
        (set `self.state` "NewEnumerator3")
        (bind _astutorial_text (cast `/Game/BluePrints/tutorial_text` (`WidgetComponent.GetUserWidgetObject` (`self.Widgettext`))))
        (`/Game/BluePrints/tutorial_text.changeText` _astutorial_text 2)))))

(event `StateTurnLeft`
  (bind _astutorial_ui (cast `/Game/BluePrints/TutorialUI` (`WidgetComponent.GetUserWidgetObject` (`self.Widget`))))
  (bind _astutorial_side (cast `/Game/BluePrints/tutorial_side` (`WidgetComponent.GetUserWidgetObject` (`self.Widgetside`))))
  (`|ExecutionSequence`
    (:`then_0`
      (`KismetSystemLibrary.Delay` 1.5)
      (bind _newparam (`self.Turnleft`))
      (set `self.leftflag` _newparam))
    (:`then_1`
      (if (`self.leftflag`)
        (`/Game/BluePrints/TutorialUI.ChangeImageState` _astutorial_ui "NewEnumerator1")
        (`/Game/BluePrints/tutorial_side.ChangeImageState` _astutorial_side "NewEnumerator1")
        (`KismetSystemLibrary.Delay` 2.0)
        (`/Game/BluePrints/TutorialUI.ChangeImageState` _astutorial_ui "NewEnumerator0")
        (`/Game/BluePrints/TutorialUI.ChangeImage` _astutorial_ui 5)
        (`/Game/BluePrints/tutorial_side.ChangeImageState` _astutorial_side "NewEnumerator0")
        (`/Game/BluePrints/tutorial_side.changeImage` _astutorial_side 5)
        (set `self.state` "NewEnumerator4")
        (bind _astutorial_text (cast `/Game/BluePrints/tutorial_text` (`WidgetComponent.GetUserWidgetObject` (`self.Widgettext`))))
        (`/Game/BluePrints/tutorial_text.changeText` _astutorial_text 3)))))

(event `StateTurnRight`
  (bind _astutorial_ui (cast `/Game/BluePrints/TutorialUI` (`WidgetComponent.GetUserWidgetObject` (`self.Widget`))))
  (bind _astutorial_side (cast `/Game/BluePrints/tutorial_side` (`WidgetComponent.GetUserWidgetObject` (`self.Widgetside`))))
  (`|ExecutionSequence`
    (:`then_0`
      (`KismetSystemLibrary.Delay` 1.5)
      (bind _newparam (`self.Turnright`))
      (set `self.rightflag` _newparam))
    (:`then_1`
      (if (`self.rightflag`)
        (`/Game/BluePrints/TutorialUI.ChangeImageState` _astutorial_ui "NewEnumerator1")
        (`/Game/BluePrints/tutorial_side.ChangeImageState` _astutorial_side "NewEnumerator1")
        (`KismetSystemLibrary.Delay` 2.0)
        (`/Game/BluePrints/TutorialUI.ChangeImageState` _astutorial_ui "NewEnumerator0")
        (`/Game/BluePrints/tutorial_side.ChangeImageState` _astutorial_side "NewEnumerator0")
        (bind _asinstance_score (cast `/Game/BluePrints/Instance_Score` (`GameplayStatics.GetGameInstance`)))
        (set `/Game/BluePrints/Instance_Score.IsFade` true _asinstance_score)
        (`KismetSystemLibrary.Delay` 3.0)
        (`GameplayStatics.OpenLevelBySoftObjectPtr` "/Game/Level/sougen.sougen")))))

(fn `callRoop3Image`
  (params (NewParam :type Integer) (NewParam1 :type Integer) (NewParam2 :type Integer))
  (bind _astutorial_ui (cast `/Game/BluePrints/TutorialUI` (`WidgetComponent.GetUserWidgetObject` (`self.Widget`))))
  (`/Game/BluePrints/TutorialUI.roop3image` _astutorial_ui NewParam NewParam1 NewParam2)
  (bind _astutorial_side (cast `/Game/BluePrints/tutorial_side` (`WidgetComponent.GetUserWidgetObject` (`self.Widgetside`))))
  (`/Game/BluePrints/tutorial_side.Roop3Image` _astutorial_side NewParam NewParam1 NewParam2))

(fn `callRoopImage`
  (params (image1 :type Integer) (image2 :type Integer))
  (bind _astutorial_ui (cast `/Game/BluePrints/TutorialUI` (`WidgetComponent.GetUserWidgetObject` (`self.Widget`))))
  (`/Game/BluePrints/TutorialUI.roop2Image` _astutorial_ui image1 image2))

(fn `Dont Move`
  (returns (NewParam :type Boolean))
  (`|ExecutionSequence`
    (:`then_0`
      ;[1 1 1] コントローラーの移動量を取得する
      (bind _asvrpawn (cast `/Game/VRTemplate/Blueprints/VRPawn` (`GameplayStatics.GetPlayerPawn` 0)))
      (`|ExecutionSequence`
        (:`then_0`
          (bind (_relativelocation_x _relativelocation_y _relativelocation_z) (`KismetMathLibrary.BreakVector` (`SceneComponent.RelativeLocation` (`/Game/VRTemplate/Blueprints/VRPawn.MotionControllerLeftAim` _asvrpawn))))
          (set `self.LeftMovementZ` (* (- _relativelocation_z (`self.LeftPositionZ`)) 5.0)))
        (:`then_1`
          (set `self.LeftPositionZ` _relativelocation_z))
        (:`then_2`
          (bind (_relativelocation_x_2 _relativelocation_y_2 _relativelocation_z_2) (`KismetMathLibrary.BreakVector` (`SceneComponent.RelativeLocation` (`/Game/VRTemplate/Blueprints/VRPawn.MotionControllerRightAim` _asvrpawn))))
          (set `self.RightMovementZ` (* (- _relativelocation_z_2 (`self.RightPositionZ`)) 5.0)))
        (:`then_3`
          (set `self.RightPositionZ` _relativelocation_z_2))))
    (:`then_1`
      ;[1 1 1] コントローラーの移動量をもとに上昇させる
      (return (and (> (`self.LeftMovementZ`) -5.0) (> (`self.RightMovementZ`) -5.0))))))

(fn `flap`
  (returns (NewParam :type Boolean))
  (`|ExecutionSequence`
    (:`then_0`
      ;[1 1 1] コントローラーの移動量を取得する
      (bind _asvrpawn (cast `/Game/VRTemplate/Blueprints/VRPawn` (`GameplayStatics.GetPlayerPawn` 0)))
      (`|ExecutionSequence`
        (:`then_0`
          (bind (_relativelocation_x _relativelocation_y _relativelocation_z) (`KismetMathLibrary.BreakVector` (`SceneComponent.RelativeLocation` (`/Game/VRTemplate/Blueprints/VRPawn.MotionControllerLeftAim` _asvrpawn))))
          (set `self.LeftMovementZ` (* (- _relativelocation_z (`self.LeftPositionZ`)) 5.0)))
        (:`then_1`
          (set `self.LeftPositionZ` _relativelocation_z))
        (:`then_2`
          (bind (_relativelocation_x_2 _relativelocation_y_2 _relativelocation_z_2) (`KismetMathLibrary.BreakVector` (`SceneComponent.RelativeLocation` (`/Game/VRTemplate/Blueprints/VRPawn.MotionControllerRightAim` _asvrpawn))))
          (set `self.RightMovementZ` (* (- _relativelocation_z_2 (`self.RightPositionZ`)) 5.0)))
        (:`then_3`
          (set `self.RightPositionZ` _relativelocation_z_2))))
    (:`then_1`
      ;[1 1 1] コントローラーの移動量をもとに上昇させる
      (return (and (< (`self.LeftMovementZ`) -5.0) (< (`self.RightMovementZ`) -5.0))))))

(fn `Turnleft`
  (returns (NewParam :type Boolean))
  (bind (_posdiffence_x _posdiffence_y _posdiffence_z) (`KismetMathLibrary.BreakVector` (`self.posDiffence`)))
  (`|ExecutionSequence`
    (:`then_0`
      ;[1 1 1] 右手と左手の差を取得
      (bind _asvrpawn (cast `/Game/VRTemplate/Blueprints/VRPawn` (`GameplayStatics.GetPlayerPawn` 0)))
      (set `self.posDiffence` (- (`SceneComponent.RelativeLocation` (`/Game/VRTemplate/Blueprints/VRPawn.MotionControllerLeftAim` _asvrpawn)) (`SceneComponent.RelativeLocation` (`/Game/VRTemplate/Blueprints/VRPawn.MotionControllerRightAim` _asvrpawn)))))
    (:`then_1`
      ;[1 1 1] 旋回
      (return (> (`KismetMathLibrary.DegAtan2` _posdiffence_z (`KismetMathLibrary.Sqrt` (+ (`KismetMathLibrary.Square` _posdiffence_x) (`KismetMathLibrary.Square` _posdiffence_y)))) 10.0)))))

(fn `Turnright`
  (returns (NewParam :type Boolean))
  (bind (_posdiffence_x _posdiffence_y _posdiffence_z) (`KismetMathLibrary.BreakVector` (`self.posDiffence`)))
  (`|ExecutionSequence`
    (:`then_0`
      ;[1 1 1] 右手と左手の差を取得
      (bind _asvrpawn (cast `/Game/VRTemplate/Blueprints/VRPawn` (`GameplayStatics.GetPlayerPawn` 0)))
      (set `self.posDiffence` (- (`SceneComponent.RelativeLocation` (`/Game/VRTemplate/Blueprints/VRPawn.MotionControllerLeftAim` _asvrpawn)) (`SceneComponent.RelativeLocation` (`/Game/VRTemplate/Blueprints/VRPawn.MotionControllerRightAim` _asvrpawn)))))
    (:`then_1`
      ;[1 1 1] 旋回
      (return (< (`KismetMathLibrary.DegAtan2` _posdiffence_z (`KismetMathLibrary.Sqrt` (+ (`KismetMathLibrary.Square` _posdiffence_x) (`KismetMathLibrary.Square` _posdiffence_y)))) -10.0)))))

(fn `UserConstructionScript`)