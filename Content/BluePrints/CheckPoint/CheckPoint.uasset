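; Checkpoint ring actor that awards score according to how close the VR pawn passes to its center.
; On overlap, it measures the pawn's Y/Z-plane offset, compares it to half the box's Y extent, and adds tiered points to Instance_Score.
; It then plays a checkpoint sound at the camera and hides the ring.
; The overlap does not check the other actor, and nothing shown disables repeat scoring.
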(event `self.ReceiveBeginPlay`
  (bind (_returnvalue_x _returnvalue_y) (`KismetMathLibrary.BreakVector` (`BoxComponent.GetScaledBoxExtent` (`self.Box`))))
  (`self.EnableInput` (`GameplayStatics.GetPlayerController` 0))
  (set `self.Max_distance` (`KismetMathLibrary.FTrunc` (/ _returnvalue_y 2.0))))

(event `self.ReceiveActorBeginOverlap`
  (params (OtherActor :type "Actor Object Reference"))
  (bind _newparam (`self.distance_calculation`))
  (bind _asinstance_score (cast `/Game/BluePrints/Instance_Score` (`GameplayStatics.GetGameInstance`)))
  (bind _returnvalue (/ _newparam (`self.Max_distance`)))
  (if (<= _returnvalue 0.2)
    (set `/Game/BluePrints/Instance_Score.AddScore` 100 _asinstance_score)
    (elif (<= _returnvalue 0.5)
      (set `/Game/BluePrints/Instance_Score.AddScore` 80 _asinstance_score)
      (elif (<= _returnvalue 1.0)
        (set `/Game/BluePrints/Instance_Score.AddScore` 50 _asinstance_score)
        (else
          (set `/Game/BluePrints/Instance_Score.AddScore` 30 _asinstance_score)))))
  (set `/Game/BluePrints/Instance_Score.Score` (+ (`/Game/BluePrints/Instance_Score.Score` _asinstance_score) (`/Game/BluePrints/Instance_Score.AddScore` _asinstance_score)) _asinstance_score)
  (`GameplayStatics.PlaySoundAtLocation` "/Game/Sounds/MSS_チェックポイント.MSS_チェックポイント" (`PlayerCameraManager.GetCameraLocation` (`GameplayStatics.GetPlayerCameraManager` 0)) (struct) 1.0 1.0 0.0 null null null null)
  (set `self.bGenerateOverlapEventsDuringLevelStreaming` false)
  (`SceneComponent.SetVisibility` (`self.ring1`) false false))

(fn `distance_calculation`
  (returns (NewParam :type "Float (double-precision)"))
  (bind (_returnvalue_x _returnvalue_y _returnvalue_z) (`KismetMathLibrary.BreakVector` (`self.K2_GetActorLocation`)))
  (bind _asvrpawn (cast `/Game/VRTemplate/Blueprints/VRPawn` (`GameplayStatics.GetPlayerPawn` 0)))
  (bind (_returnvalue_x_2 _returnvalue_y_2 _returnvalue_z_2) (`KismetMathLibrary.BreakVector` (`self.K2_GetActorLocation` _asvrpawn)))
  (return (`KismetMathLibrary.Sqrt` (+ (`KismetMathLibrary.Square` (- _returnvalue_y_2 _returnvalue_y)) (`KismetMathLibrary.Square` (- _returnvalue_z_2 _returnvalue_z))))))

(fn `UserConstructionScript`)