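; Instance_Score is a Blueprint that controls a post-process fade, with no score logic in these graphs.
; FadeSystem steps FadeVal by ChangeFadeVal per call, up or down according to IsFade, with bounds checked before each step rather than clamped.
; Fade separately writes FadeVal to the FadeOpacity scalar in the MPC_PostProcess material parameter collection.
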(fn `Fade`
  (`KismetMaterialLibrary.SetScalarParameterValue` "/Game/Material/MPC_PostProcess.MPC_PostProcess" "FadeOpacity" (`self.FadeVal`)))

(fn `FadeSystem`
  (if (`self.IsFade`)
    (if (<= (`self.FadeVal`) 1.0)
      (set `self.FadeVal` (+ (`self.FadeVal`) (`self.ChangeFadeVal`))))
    (elif (>= (`self.FadeVal`) 0.0)
      (set `self.FadeVal` (- (`self.FadeVal`) (`self.ChangeFadeVal`))))))