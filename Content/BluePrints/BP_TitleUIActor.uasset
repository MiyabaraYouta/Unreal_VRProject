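; BP_TitleUIActor is a title UI actor that blinks its UIPlease component, likely a prompt.
; BeginPlay hides UIPlease, reveals it after a six-second delay and sets IsTimeLoop to start the blinking.
; While the flag is set, Tick drives chained latent Delays that repeatedly hide and show UIPlease, relying on Delay ignoring calls while pending instead of using a timer.
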(event `self.ReceiveBeginPlay`
  (`SceneComponent.SetVisibility` (`self.UI_Please`) false false)
  (`KismetSystemLibrary.Delay` 6.0)
  (`SceneComponent.SetVisibility` (`self.UI_Please`) true false)
  (set `self.IsTimeLoop` true))

(event `self.ReceiveTick`
  (params (DeltaSeconds :type "Float (single-precision)"))
  (bind _ui_please (`self.UI_Please`))
  (if (`self.IsTimeLoop`)
    (`KismetSystemLibrary.Delay` 2.0)
    (`SceneComponent.SetVisibility` _ui_please false false)
    (`KismetSystemLibrary.Delay` 0.6)
    (`SceneComponent.SetVisibility` _ui_please true false)))

(fn `UserConstructionScript`)