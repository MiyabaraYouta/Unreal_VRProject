(event `self.ReceiveBeginPlay`
  (`KismetSystemLibrary.Delay` 4.0)
  (set `self.IsCharacterViw` true))

(event `self.ReceiveTick`
  (params (DeltaSeconds :type "Float (single-precision)"))
  (if (`self.IsCharacterViw`)
    (`KismetSystemLibrary.Delay` 2.0)
    (`SceneComponent.SetVisibility` (`self.Text_ThankYou`) false false)
    (`KismetSystemLibrary.Delay` 0.6)
    (`SceneComponent.SetVisibility` (`self.Text_ThankYou`) true false)))

(fn `UserConstructionScript`)