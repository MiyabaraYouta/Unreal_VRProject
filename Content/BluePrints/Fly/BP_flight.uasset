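; BP_flight gives the VR player wing-flap flight along the HMD's forward direction.
; Each tick it derives vertical velocity of both controllers; a fast simultaneous downstroke plays a flap sound and resets speed, re-armed by an upstroke.
; Speed moves the pawn, decays every frame, and drives speed-line post-process opacity, plus wind audio in two levels.
; On/Off events set IsActive, but nothing live reads it.
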(event `self.ReceiveTick`
  (params (DeltaSeconds :type "Float (single-precision)"))
  (bind _rightmovementz (`self.RightMovementZ`))
  (bind _leftmovementz (`self.LeftMovementZ`))
  (`|ExecutionSequence`
    (:`then_0`
      ;[1 1 1] コントローラーの移動量を取得する
      (bind _asvrpawn (cast `/Game/VRTemplate/Blueprints/VRPawn` (`GameplayStatics.GetPlayerPawn` 0)))
      (`|ExecutionSequence`
        (:`then_0`
          (bind (_relativelocation_x _relativelocation_y _relativelocation_z) (`KismetMathLibrary.BreakVector` (`SceneComponent.RelativeLocation` (`/Game/VRTemplate/Blueprints/VRPawn.MotionControllerLeftAim` _asvrpawn))))
          (set `self.LeftMovementZ` (/ (- _relativelocation_z (`self.LeftPositionZ`)) DeltaSeconds)))
        (:`then_1`
          (set `self.LeftPositionZ` _relativelocation_z))
        (:`then_2`
          (bind (_relativelocation_x_2 _relativelocation_y_2 _relativelocation_z_2) (`KismetMathLibrary.BreakVector` (`SceneComponent.RelativeLocation` (`/Game/VRTemplate/Blueprints/VRPawn.MotionControllerRightAim` _asvrpawn))))
          (set `self.RightMovementZ` (/ (- _relativelocation_z_2 (`self.RightPositionZ`)) DeltaSeconds)))
        (:`then_3`
          (set `self.RightPositionZ` _relativelocation_z_2))))
    (:`then_1`
      (`self.turn`)
      (`self.advance`)
      (`self.deceleration`))
    (:`then_2`
      ;[1 1 1] コントローラーの移動量をもとに上昇させる
      (if (and (< _leftmovementz -50.0) (< _rightmovementz -50.0))
        (if (`self.soundFlag`)
          (`GameplayStatics.PlaySoundAtLocation` "/Game/Sounds/habataki/MSS_羽ばたき.MSS_羽ばたき" (`PlayerCameraManager.GetCameraLocation` (`GameplayStatics.GetPlayerCameraManager` 0)) (struct) 1.0 1.0 0.0 null null null null)
          (set `self.soundFlag` false)
          (`self.flap`))))
    (:`then_3`
      (if (and (> _rightmovementz 50.0) (> _leftmovementz 50.0))
        (set `self.soundFlag` true)))))

(event `/Game/BluePrints/Interface/IVRPorn.OffFlySystem`
  (set `self.IsActive` false))

(event `/Game/BluePrints/Interface/IVRPorn.OnFlySystem`
  (set `self.IsActive` true))

(fn `advance`
  (bind _asvrpawn (cast `/Game/VRTemplate/Blueprints/VRPawn` (`GameplayStatics.GetPlayerPawn` 0)))
  (`self.K2_AddActorWorldTransform` _asvrpawn (`KismetMathLibrary.MakeTransform` (* (`self.HMDForwardVector`) (`self.speed`))) false false))

(fn `deceleration`
  (if (> (`self.speed`) 0.0)
    (bind _output_get (set `self.speed` (* (`self.speed`) 0.995)))
    (bind _returnvalue (`GameplayStatics.GetCurrentLevelName` true))
    (bind _returnvalue_2 (/ _output_get 100.0))
    (`KismetMaterialLibrary.SetScalarParameterValue` "/Game/SpeedLine/MPC_PostProcess_SpeedLine.MPC_PostProcess_SpeedLine" "SpeedLineOpacity" _returnvalue_2)
    (if (or (`KismetStringLibrary.EqualEqual_StrStr` _returnvalue "sougen") (`KismetStringLibrary.EqualEqual_StrStr` _returnvalue "setugen"))
      (`AudioParameterControllerInterface.SetFloatParameter` (`self.MSS_Audio`) "WindStrengs" _returnvalue_2))))

(fn `flap`
  (set `self.speed` 100.0))

(fn `turn`
  (bind _asvrpawn (cast `/Game/VRTemplate/Blueprints/VRPawn` (`GameplayStatics.GetPlayerPawn` 0)))
  (set `self.HMDForwardVector` (`KismetMathLibrary.GetForwardVector` (`SceneComponent.K2_GetComponentRotation` (`/Game/VRTemplate/Blueprints/VRPawn.Camera` _asvrpawn)))))

(fn `UserConstructionScript`)