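; BP_Pitch is a flight-control Blueprint that pitches the player's VRPawn from motion controller rotation.
; Each Tick reads both aim controllers' roll, offset by 90 degrees in opposite directions with a five-degree dead zone.
; Mirrored twists of both hands add a fixed one-degree local pitch step up or down, independent of delta time.
; Draft logic for limiting pitch to 45 degrees either way is unconnected and never runs.
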(event `self.ReceiveTick`
  (params (DeltaSeconds :type "Float (single-precision)"))
  (`|ExecutionSequence`
    (:`then_0`
      (bind _asvrpawn (cast `/Game/VRTemplate/Blueprints/VRPawn` (`GameplayStatics.GetPlayerPawn` 0)))
      (bind _relativerotation_roll (`KismetMathLibrary.BreakRotator` (`SceneComponent.RelativeRotation` (`/Game/VRTemplate/Blueprints/VRPawn.MotionControllerLeftAim` _asvrpawn))))
      (bind _returnvalue (- _relativerotation_roll 90.0))
      (bind _relativerotation_roll_2 (`KismetMathLibrary.BreakRotator` (`SceneComponent.RelativeRotation` (`/Game/VRTemplate/Blueprints/VRPawn.MotionControllerRightAim` _asvrpawn))))
      (bind _returnvalue_2 (+ _relativerotation_roll_2 90.0))
      (if (and (and (< _returnvalue -5.0) (> _returnvalue -180.0)) (and (> _returnvalue_2 5.0) (< _returnvalue_2 180.0)))
        (if true
          (`self.K2_AddActorLocalTransform` _asvrpawn (`KismetMathLibrary.MakeTransform` (0.0 0.0 0.0) (`KismetMathLibrary.MakeRotator` 0.0 -1.0)) false false))
        (elif (and (or (> _returnvalue 5.0) (< _returnvalue -180.0)) (or (< _returnvalue_2 -5.0) (> _returnvalue_2 180.0)))
          (if true
            (`self.K2_AddActorLocalTransform` _asvrpawn (`KismetMathLibrary.MakeTransform` (0.0 0.0 0.0) (`KismetMathLibrary.MakeRotator` 0.0 1.0)) false false)))))))

(fn `UserConstructionScript`)