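; BP_Turn steers the VR pawn in the flight system by tilting the hands, yawing it by the controllers' height difference.
; Each Tick measures the tilt between left and right aim controllers, turning only beyond a small dead zone.
; The tilt also picks a three-state Funstr value, passed through a condition and delay to AudinoTest_BP's SendSerial.
; On/Off FlySystem events set IsActive, but Tick never checks it.
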(event `self.ReceiveTick`
  (params (DeltaSeconds :type "Float (single-precision)"))
  (bind (_posdiffence_x _posdiffence_y _posdiffence_z) (`KismetMathLibrary.BreakVector` (`self.posDiffence`)))
  (bind (_posdiffence_x_2 _posdiffence_y_2 _posdiffence_z_2) (`KismetMathLibrary.BreakVector` (`self.posDiffence`)))
  (bind (_posdiffence_x_3 _posdiffence_y_3 _posdiffence_z_3) (`KismetMathLibrary.BreakVector` (`self.posDiffence`)))
  (bind _returnvalue (`KismetMathLibrary.DegAtan2` _posdiffence_z_2 (`KismetMathLibrary.Sqrt` (+ (`KismetMathLibrary.Square` _posdiffence_x_2) (`KismetMathLibrary.Square` _posdiffence_y_2)))))
  (bind _returnvalue_2 (`KismetMathLibrary.DegAtan2` _posdiffence_z (`KismetMathLibrary.Sqrt` (+ (`KismetMathLibrary.Square` _posdiffence_x) (`KismetMathLibrary.Square` _posdiffence_y)))))
  (bind _returnvalue_3 (< _returnvalue -10.0))
  (bind _returnvalue_4 (> _returnvalue 10.0))
  (`|ExecutionSequence`
    (:`then_0`
      ;[1 1 1] 右手と左手の差を取得
      (bind _asvrpawn (cast `/Game/VRTemplate/Blueprints/VRPawn` (`GameplayStatics.GetPlayerPawn` 0)))
      (set `self.posDiffence` (- (`SceneComponent.RelativeLocation` (`/Game/VRTemplate/Blueprints/VRPawn.MotionControllerLeftAim` _asvrpawn)) (`SceneComponent.RelativeLocation` (`/Game/VRTemplate/Blueprints/VRPawn.MotionControllerRightAim` _asvrpawn)))))
    (:`then_1`
      ;[1 1 1] 旋回
      (bind _asvrpawn_2 (cast `/Game/VRTemplate/Blueprints/VRPawn` (`GameplayStatics.GetPlayerPawn` 0)))
      (if (or (< _returnvalue_2 -10.0) (> _returnvalue_2 10.0))
        (`self.K2_AddActorWorldRotation` _asvrpawn_2 (`KismetMathLibrary.MakeRotator` 0.0 0.0 (/ _posdiffence_z_3 100.0)) false false)))
    (:`then_2`
      (bind _outactors (`GameplayStatics.GetAllActorsOfClass` "/Game/BluePrints/Audino/AudinoTest_BP.AudinoTest_BP_C"))
      (`|ExecutionSequence`
        (:`then_0`
          (if _returnvalue_3
            (set `self.funstr` "NewEnumerator5")
            (elif _returnvalue_4
              (set `self.funstr` "NewEnumerator15")
              (else
                (set `self.funstr` "NewEnumerator4")))))
        (:`then_1`
          (if (`KismetMathLibrary.BooleanNAND` (and _returnvalue_3 (`|EnumEquality` (`self.funstr`) "NewEnumerator5")) (and _returnvalue_4 (`|EnumEquality` (`self.funstr`) "NewEnumerator15")) (and (`KismetMathLibrary.BooleanNAND` _returnvalue_3 _returnvalue_4) (`|EnumEquality` (`self.funstr`) "NewEnumerator4")))
            (`KismetSystemLibrary.Delay` 1.0)
            (`/Game/BluePrints/Audino/AudinoTest_BP.SendSerial` _outactors (`self.funstr`))))))))

(event `/Game/BluePrints/Interface/IVRPorn.OffFlySystem`
  (set `self.IsActive` false)
  (`KismetSystemLibrary.PrintString` "Hello" :!label _label))

(event `/Game/BluePrints/Interface/IVRPorn.OnFlySystem`
  (set `self.IsActive` true)
  (goto _label))

(fn `UserConstructionScript`)