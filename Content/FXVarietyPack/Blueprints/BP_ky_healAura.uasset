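; BP_ky_healAura is an effect actor from FXVarietyPack, named as a heal aura, that travels along the level's FlyingPath actor.
; Its construction script looks up that path and copies its start and end segment and point.
; Each tick it passes itself, a fixed speed and delta time to the path's MoveForwardClass, stores the returned position indices, and destroys itself upon reaching the end.
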(event `self.ReceiveBeginPlay`
  (`parent.ReceiveBeginPlay`))

(event `self.ReceiveTick`
  (params (DeltaSeconds :type "Float (single-precision)"))
  (`parent.ReceiveTick` DeltaSeconds)
  (bind _returnvalue (`GameplayStatics.GetActorOfClass` "/Script/Unreal_VRProject.FlyingPath"))
  (bind (_outnewsegment _outcurpoint) (`FlyingPath.MoveForwardClass` _returnvalue (`self.currentSegment`) 500.0 self DeltaSeconds))
  (set `self.currentSegment` _outnewsegment)
  (set `self.currentPoint` _outcurpoint)
  (if (and (>= (`self.currentPoint`) (`self.endPoint`)) (>= (`self.currentSegment`) (`self.endSegment`)))
    (`self.K2_DestroyActor`)))

(fn `UserConstructionScript`
  (`parent.UserConstructionScript`)
  (bind _returnvalue (`GameplayStatics.GetActorOfClass` "/Script/Unreal_VRProject.FlyingPath"))
  (set `self.endSegment` (`FlyingPath.endSegment` _returnvalue))
  (set `self.endPoint` (`FlyingPath.endPoint` _returnvalue))
  (set `self.currentSegment` (`FlyingPath.startSegment` _returnvalue))
  (set `self.currentPoint` (`FlyingPath.startPoint` _returnvalue)))